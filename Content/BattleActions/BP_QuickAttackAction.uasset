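; Battle action for a quick sword attack that locks the owner's movement while it plays.
; Execute toggles lock-on, shows the sword with collision, overlap events and a light, then a timeline yaws the turn point to swing it.
; The swing ends on completion, when ExecutionTime is reached or after DeActivate clears the uninterrupted flag.
; Cleanup hides the sword, disables collision and light, restores walking and toggles lock-on back.
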(event EventBeginPlay
  (|CallParentFunction)
  (CallFunction|SetCollisionandTrigger false "NoCollision"))

(event EventExecute
  ;[1 0.857 0.3604] execute action
  (CallFunction|ToggleLockon)
  (CallFunction|Activation)
  (bind (_direction _angle _time) (Timeline|swing PlayFromStart)
    (:Update
      (bind _timelinetolong (CallFunction|InteruptAction _time))
      (if _timelinetolong
        (Utilities|FlowControl|Sequence
          (:then_0
            (Timeline|swing Stop))
          (:then_1
            ;[1 0.9349 0.2192] clean up
            (CallFunction|Finish :!label _label)
            (CallFunction|ToggleLockon)))
        (else
          (Transformation|SetRelativeRotation (Variables|Default|Getturnpoint) (Math|Rotator|MakeRotator 0.0 0.0 _angle) false false))))
    (:Finished
      (goto _label))))

(event EventDeActivate
  ;[1 0.7569 0.321] deactivate action
  (Variables|Default|SetunInterupted false))

(fn ConstructionScript)

(fn InteruptAction
  (params (deltatime :type Float%20%28double-precision%29))
  (return (or (>= deltatime (Variables|Default|GetExecutionTime)) (not (Variables|Default|GetunInterupted)))))

(fn Finish
  (bind _returnvalue (Class|BattleActionBase|GetParentMovementComp))
  (Rendering|Components|Light|SetIntensity (Variables|Default|GetPointLight) 0.0)
  (CallFunction|SetCollisionandTrigger false "NoCollision")
  ;[1 1 1] enable movement again
  (Utilities|IsValid _returnvalue
    (:Is%20Valid
      (Pawn|Components|CharacterMovement|SetMovementMode _returnvalue "MOVE_Walking" 0))))

(fn SetCollisionandTrigger
  (params (generate%20event :type Boolean) (collisionType :type ECollisionEnabled%20Enum :default "NoCollision"))
  (bind _output_get (Variables|/Script/Engine.PrimitiveComponent|SetbGenerateOverlapEvents (Variables|Default|GettriggerCaps) generate%20event))
  (Rendering|SetVisibility (Variables|Default|Getsword) _output_get false)
  (Collision|SetCollisionEnabled (Variables|Default|Getsword) collisionType))

(fn Activation
  (bind _returnvalue (Class|BattleActionBase|GetParentMovementComp))
  (Variables|Default|SetunInterupted true)
  (CallFunction|SetCollisionandTrigger true "QueryAndPhysics")
  (Rendering|Components|Light|SetIntensity (Variables|Default|GetPointLight) (Variables|Default|GetlightIntensity))
  ;[1 1 1] disable movement again
  (Utilities|IsValid _returnvalue
    (:Is%20Valid
      (Pawn|Components|CharacterMovement|DisableMovement _returnvalue))))