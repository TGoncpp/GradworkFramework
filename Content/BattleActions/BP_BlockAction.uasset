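; Battle action actor for blocking that shows a guard by toggling a point light and scaling a Guard component.
; Execute turns the light on and scales Guard to its active size; DeActivate turns it off and shrinks Guard to its inactive size, both with swept transforms.
; The light starts off at BeginPlay.
; A timed BlockTime countdown with guard helper functions exists but is disconnected, and Tick is empty.
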(event EventBeginPlay
  (Rendering|Components|Light|SetIntensity (Variables|Default|GetPointLight) 0.0))

(event Collision|EventActorBeginOverlap
  (params (OtherActor :type Actor%20Object%20Reference)))

(event EventTick
  (params (DeltaSeconds :type Float%20%28single-precision%29))
  ;[1 1 1] Activate block
)

(event EventExecute
  ;[1 0.7719 0.1777] execute attack
  (Rendering|Components|Light|SetIntensity (Variables|Default|GetPointLight) (Variables|actionSettings|GetlightIntensity))
  (Transformation|SetRelativeTransform (Variables|Default|Getguard) (Math|Transform|MakeTransform "0, 0, 0" "0, 0, 0" (Math|Conversions|ToVector(Float) (Variables|Default|GetactiveSize))) true false))

(event EventDeActivate
  ;[1 0.848 0.2119] deactivate
  (Rendering|Components|Light|SetIntensity (Variables|Default|GetPointLight) 0.0)
  (Transformation|SetRelativeTransform (Variables|Default|Getguard) (Math|Transform|MakeTransform "0, 0, 0" "0, 0, 0" (Math|Conversions|ToVector(Float) (Variables|Default|GetDeActiveSize))) true false))

(fn ConstructionScript)

(fn UpdateLight
  (params (InputPin :type Float%20%28single-precision%29))
  (bind _pointlight (Variables|Default|GetPointLight))
  (if (> (Variables|actionSettings|GetblockTime) 0.0)
    (Variables|actionSettings|SetblockTime (- (Variables|actionSettings|GetblockTime) InputPin))
    (Rendering|Components|Light|SetIntensity _pointlight (Variables|actionSettings|GetlightIntensity))
    (return false)
    (else
      (Rendering|Components|Light|SetIntensity _pointlight 0.0)
      (return true))))

(fn ActivateGuard
  (Transformation|SetRelativeTransform (Variables|Default|Getguard) (Math|Transform|MakeTransform "0, 0, 0" "0, 0, 0" (Math|Conversions|ToVector(Float) (Variables|Default|GetactiveSize))) true false))

(fn DeactivateGuard
  (Transformation|SetRelativeTransform (Variables|Default|Getguard) (Math|Transform|MakeTransform "0, 0, 0" "0, 0, 0" (Math|Conversions|ToVector(Float) (Variables|Default|GetDeActiveSize))) true false))