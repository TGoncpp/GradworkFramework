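; BP_HealAction is a battle action that heals its parent BP_Hero after a visible channeling period.
; Execute turns on a point light and shows a heal circle, whose height the Heal timeline animates.
; When the timeline finishes without interruption, Recover calls the hero's HealthComponent to restore health, then hides the effects.
; DeActivate clears the uninterrupted flag and hides the effects immediately, so the pending heal is skipped.
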(event EventBeginPlay)

(event Collision|EventActorBeginOverlap
  (params (OtherActor :type Actor%20Object%20Reference)))

(event EventTick
  (params (DeltaSeconds :type Float%20%28single-precision%29)))

(event EventExecute
  ;[1 0.857 0.3604] execute action
  (Variables|Default|SetunInterupted true)
  (Rendering|Components|Light|SetIntensity (Variables|Default|GetPointLight) (Variables|Default|Getlightintensity))
  (Rendering|SetVisibility (Variables|Default|GethealCirlce) true false)
  (bind _newtrack_0 (Timeline|heal PlayFromStart)
    (:Update
      (Transformation|SetRelativeLocation (Variables|Default|GethealCirlce) (Math|Vector|MakeVector 0.0 0.0 _newtrack_0) true false))
    (:Finished
      ;[0.3735 1 0.2551] On finish heal
      (if (Variables|Default|GetunInterupted)
        (CallFunction|Recover)
        (Rendering|Components|Light|SetIntensity (Variables|Default|GetPointLight) 0.0)
        (Rendering|SetVisibility (Variables|Default|GethealCirlce) false false)))))

(event EventDeActivate
  ;[1 0.7286 0.3673] On deactivate
  (Variables|Default|SetunInterupted false)
  (Rendering|Components|Light|SetIntensity (Variables|Default|GetPointLight) 0.0)
  (Rendering|SetVisibility (Variables|Default|GethealCirlce) false false))

(fn ConstructionScript)

(fn Recover
  (bind _asbp_hero (Utilities|Casting|CastToBP_Hero (Class|BattleActionBase|GetParent)))
  (Utilities|IsValid (Actor|GetComponentbyClass _asbp_hero "/Script/Gradwork_npcAI.HealthComponent")
    (:Is%20Valid
      (Class|HealthComponent|Recover (Actor|GetComponentbyClass _asbp_hero "/Script/Gradwork_npcAI.HealthComponent")))))