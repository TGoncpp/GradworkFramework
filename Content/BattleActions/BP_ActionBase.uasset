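; BP_ActionBase is a base Blueprint for battle actions that operate on the character they are attached to.
; ToggleLockOn casts the parent to BP_Hero and calls its LockOn function.
; OnAttachToCharact, commented as creating a parent reference, only validates the parent and its CharacterMovementComponent, with no logic after the checks.
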(fn ConstructionScript)

(fn OnAttachtoCharact
  (bind _returnvalue (Class|BattleActionBase|GetParent))
  ;[1 1 1] create parent refrence
  (Utilities|IsValid _returnvalue
    (:Is%20Valid
      (Utilities|IsValid (Actor|GetComponentbyClass _returnvalue "/Script/Engine.CharacterMovementComponent")))))

(fn ToggleLockon
  (bind _returnvalue (Class|BattleActionBase|GetParent))
  (Utilities|IsValid _returnvalue
    (:Is%20Valid
      (bind _asbp_hero (Utilities|Casting|CastToBP_Hero _returnvalue))
      (Utilities|IsValid _asbp_hero
        (:Is%20Valid
          (Class|SoulsCharacter|Lockon _asbp_hero))
        (:Is%20Not%20Valid
          _)))
    (:Is%20Not%20Valid
      _))
  (return))