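; Battle action that throws a rock forward from its owner, briefly rooting that owner and lighting a point light.
; The Throw timeline sweeps the trigger capsule along the actor's forward vector, restoring parent walking and switching off the light once ExecutionTime passes.
; Overlapping another BP_Hero or finishing the timeline hides the rock and disables its collision, with no damage applied here.
; A Test flag fires delayed throws from Tick.
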(event OnComponentBeginOverlap(triggerCaps)
  (params (OverlappedComponent :type Primitive%20Component%20Object%20Reference) (OtherActor :type Actor%20Object%20Reference) (OtherComp :type Primitive%20Component%20Object%20Reference) (OtherBodyIndex :type Integer) (bFromSweep :type Boolean) (SweepResult :type Hit%20Result%20Structure%20%28by%20ref%29))
  ;[0.4564 0.91 1] dissable collision on touch
  (if (not (or (== OtherActor self) (== OtherActor (Class|BattleActionBase|GetParent))))
    (Utilities|Casting|CastToBP_Hero OtherActor)
    (CallFunction|DeAcivation)))

(event Custom|TestThrow
  ;[1 0.857 0.3604] execute action
  (CallFunction|PrepareThrow)
  (Variables|/Script/Engine.PrimitiveComponent|SetbGenerateOverlapEvents (Variables|Default|GettriggerCaps) true)
  (bind (_direction _throwdistance _time) (Timeline|throw PlayFromStart)
    (:Update
      (CallFunction|ReAbleMovement _time)
      (Transformation|AddWorldOffset (Variables|Default|GettriggerCaps) (* (Transformation|GetActorForwardVector) _throwdistance) true false))
    (:Finished
      ;[1 1 1] clean up
      (CallFunction|DeAcivation))))

(event EventTick
  (params (DeltaSeconds :type Float%20%28single-precision%29))
  ;[1 1 1] TestShooting
  (if (Variables|Default|Gettest)
    (Utilities|FlowControl|Delay 2.0)
    (CallFunction|TestThrow)))

(event EventExecute
  ;[1 0.857 0.3604] execute action
  (CallFunction|PrepareThrow)
  (Variables|/Script/Engine.PrimitiveComponent|SetbGenerateOverlapEvents (Variables|Default|GettriggerCaps) true)
  (bind (_direction _throwdistance _time) (Timeline|throw PlayFromStart)
    (:Update
      (CallFunction|ReAbleMovement _time)
      (Transformation|AddWorldOffset (Variables|Default|GettriggerCaps) (* (Transformation|GetActorForwardVector) _throwdistance) true false))
    (:Finished
      ;[1 1 1] clean up
      (CallFunction|DeAcivation))))

(fn ConstructionScript)

(fn PrepareThrow
  (bind _returnvalue (Class|BattleActionBase|GetParentMovementComp))
  (Rendering|Components|Light|SetIntensity (Variables|Default|GetPointLight) (Variables|ActionSetting|GetLightIntensity))
  (Rendering|SetVisibility (Variables|Default|Getrock) true false)
  (Collision|SetCollisionEnabled (Variables|Default|GettriggerCaps) "QueryAndPhysics")
  ;[1 1 1] enable movement again
  (Variables|Default|SetmovementDisabled true)
  (Utilities|IsValid _returnvalue
    (:Is%20Valid
      (Pawn|Components|CharacterMovement|DisableMovement _returnvalue))))

(fn DeAcivation
  (Collision|SetCollisionEnabled (Variables|Default|GettriggerCaps) "NoCollision")
  (Rendering|SetVisibility (Variables|Default|Getrock) false false)
  (Variables|/Script/Engine.PrimitiveComponent|SetbGenerateOverlapEvents (Variables|Default|GettriggerCaps) false))

(fn ReAbleMovement
  (params (currentTime :type Float%20%28double-precision%29))
  (bind _returnvalue (Class|BattleActionBase|GetParentMovementComp))
  (if (>= currentTime (Variables|Default|GetExecutionTime))
    (if (Variables|Default|GetmovementDisabled)
      ;[1 1 1] enable movement again
      (Variables|Default|SetmovementDisabled false)
      (Utilities|IsValid _returnvalue
        (:Is%20Valid
          (Pawn|Components|CharacterMovement|SetMovementMode _returnvalue "MOVE_Walking" 0)
          (Rendering|Components|Light|SetIntensity (Variables|Default|GetPointLight) 0.0))))))