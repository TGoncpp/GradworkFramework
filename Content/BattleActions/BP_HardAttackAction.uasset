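; Battle action for a hard attack that swings a sword and enables its hit trigger while active.
; Execute or Swing shows the sword, turns on collision, overlap events and a light, then a timeline pitches the turn point.
; The timeline stops when execution time is reached or the action is deactivated; DeActivate or timeline completion hides and disables everything.
; A test flag on Tick triggers delayed repeat swings.
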(event Custom|Swing
  ;[1 0.6512 0.1707] On activation
  (CallFunction|OnActivation)
  (bind (_direction _swing _time) (Timeline|Timeline PlayFromStart)
    (:Update
      (bind _quit (CallFunction|InteruptAction _time))
      (if _quit
        (Timeline|Timeline Stop)
        (else
          (Transformation|SetRelativeRotation (Variables|Default|GetturnPoint) (Math|Rotator|MakeRotator 0.0 _swing 0.0) false false))))
    (:Finished
      (CallFunction|OnDeactivation))))

(event EventBeginPlay
  (CallFunction|SetCollisionTrigger false "NoCollision"))

(event EventTick
  (params (DeltaSeconds :type Float%20%28single-precision%29))
  ;[1 1 1] For testing
  (Utilities|FlowControl|Delay 2.0)
  (if (Variables|Default|GetDoTestSwings)
    (CallFunction|Swing)))

(event EventExecute
  ;[1 0.6512 0.1707] On activation
  (CallFunction|OnActivation)
  (bind (_direction _swing _time) (Timeline|Timeline PlayFromStart)
    (:Update
      (bind _quit (CallFunction|InteruptAction _time))
      (if _quit
        (Timeline|Timeline Stop)
        (else
          (Transformation|SetRelativeRotation (Variables|Default|GetturnPoint) (Math|Rotator|MakeRotator 0.0 _swing 0.0) false false))))
    (:Finished
      (CallFunction|OnDeactivation))))

(event EventDeActivate
  ;[1 0.6766 0.1579] On deactivate action
  (CallFunction|OnDeactivation))

(fn ConstructionScript)

(fn OnDeactivation
  (Variables|Default|SetunIntrupted false)
  (Rendering|Components|Light|SetIntensity (Variables|Default|GetPointLight) 0.0)
  (CallFunction|SetCollisionTrigger false "NoCollision"))

(fn OnActivation
  (Variables|Default|SetunIntrupted true)
  (Rendering|Components|Light|SetIntensity (Variables|Default|GetPointLight) (Variables|actionSetting|Getlightintensity))
  (CallFunction|SetCollisionTrigger true "QueryAndPhysics"))

(fn InteruptAction
  (params (time :type Float%20%28double-precision%29))
  (return (or (>= time (Variables|Default|GetExecutionTime)) (not (Variables|Default|GetunIntrupted)))))

(fn SetCollisionTrigger
  (params (trigger :type Boolean) (collisionType :type ECollisionEnabled%20Enum :default "NoCollision"))
  (bind _output_get (Variables|/Script/Engine.PrimitiveComponent|SetbGenerateOverlapEvents (Variables|Default|GettriggerCaps) trigger))
  (Rendering|SetVisibility (Variables|Default|Getsword) _output_get false)
  (Collision|SetCollisionEnabled (Variables|Default|Getsword) collisionType))